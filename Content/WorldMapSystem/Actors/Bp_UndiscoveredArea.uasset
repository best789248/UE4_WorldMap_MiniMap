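; Undiscovered area marker for the world map system, optionally shrouded in a smoke particle effect until discovered.
; The construction script sizes an area sphere and a larger discovery sphere from the area radius, scaling the smoke to match.
; The first overlap by an actor with a BpC_WorldMap component reports the area to that component.
; OnDiscovered deactivates any smoke, waits briefly, then destroys the actor.
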(event OnComponentBeginOverlap(DiscoverSphere)
  (params (OverlappedComponent :type Primitive%20Component%20Object%20Reference) (OtherActor :type Actor%20Object%20Reference) (OtherComp :type Primitive%20Component%20Object%20Reference) (OtherBodyIndex :type Integer) (bFromSweep :type Boolean) (SweepResult :type Hit%20Result%20Structure%20%28by%20ref%29))
  (bind _returnvalue (Actor|GetComponentbyClass OtherActor "/Game/WorldMapSystem/Actors/BpC_WorldMap.BpC_WorldMap_C"))
  (Utilities|IsValid _returnvalue
    (:Is%20Valid
      (Utilities|FlowControl|DoOnce false
        (:Completed
          (Default|OndiscoverArea _returnvalue self))))))

(event Custom|OnDiscovered
  (Utilities|IsValid (Variables|Default|GetParticleSystem)
    (:Is%20Valid
      (Components|Activation|Deactivate (Variables|Default|GetParticleSystem))
      (Utilities|FlowControl|Delay 2.5))
    (:Is%20Not%20Valid
      _))
  (Actor|DestroyActor))

(event EventBeginPlay
  (if (not (Variables|Setting|GetShowSmoke?))
    (Components|DestroyComponent (Variables|Default|GetParticleSystem))))

(event Collision|EventActorBeginOverlap
  (params (OtherActor :type Actor%20Object%20Reference)))

(event EventTick
  (params (DeltaSeconds :type Float%20%28single-precision%29)))

(fn ConstructionScript
  (bind _particlesystem (Variables|Default|GetParticleSystem))
  (bind _arearadius (Variables|Setting|GetAreaRadius))
  (Components|Sphere|SetSphereRadius (Variables|Default|GetAreaSphere) _arearadius false)
  (Components|Sphere|SetSphereRadius (Variables|Default|GetDiscoverSphere) (+ _arearadius (Variables|Setting|GetAdditionalDiscoverRadius)) false)
  (Transformation|SetRelativeScale3D _particlesystem (Math|Conversions|ToVector(Float) (Math|Float|Clamp(Float) (/ (Variables|Setting|GetAreaRadius) 1.5e+02) 0.1 1e+02)))
  (Rendering|SetVisibility _particlesystem (Variables|Setting|GetShowSmoke?) false))